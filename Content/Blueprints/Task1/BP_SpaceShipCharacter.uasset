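; Spaceship character for a team-based multiplayer game that colors its mesh by team and drives HUD refreshes.
; AssignMaterial calls a server event that compares the player state's team name with game state team B, choosing red or blue.
; The RepNotify on Material applies the choice to SpaceMesh.
; A looping one-second timer from BeginPlay chains through server and multi HUD events to fire player controller 0's UI update delegate.
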(event `self.AssignMaterial`
  (`self.ServerAssignmaterial`))

(event `ServerAssignmaterial`
  (bind (_asbp_space_ship_player_state _bsuccess) (cast `/Game/Blueprints/BP_SpaceShipPlayerState` (`self.PlayerState`) :!pure true))
  (bind (_asbp_space_ship_game_state_base _bsuccess_2) (cast `/Game/Blueprints/Task1/BP_SpaceShipGameStateBase` (`GameplayStatics.GetGameState`) :!pure true))
  (if (and _bsuccess _bsuccess_2)
    (if (`KismetStringLibrary.EqualEqual_StrStr` (`SpaceShipPlayerState.GetTeamName` _asbp_space_ship_player_state) (`SpaceShipGameStateBase.GetTeamName` _asbp_space_ship_game_state_base (`SpaceShipGameStateBase.TeamsStructB` _asbp_space_ship_game_state_base)))
      (set `self.Material` "/Game/TwinStick/Meshes/RedMaterial.RedMaterial")
      (else
        (set `self.Material` "/Game/TwinStick/Meshes/BlueMaterial.BlueMaterial")))))

(event `self.ReceiveBeginPlay`
  (`KismetSystemLibrary.K2_SetTimerDelegate` (delegate `ServerCAllMultiHUD`) 1.0 true))

(event `ServerCAllMultiHUD`
  (`self.MultiHUD`))

(event `MultiHUD`
  (bind _asbp_space_ship_player_controller (cast `/Game/Blueprints/Task1/BP_SpaceShipPlayerController` (`GameplayStatics.GetPlayerController` 0)))
  (`SpaceShipPlayerController.CallUpdateUIDelegate` _asbp_space_ship_player_controller))

(fn `OnRep_Material`
  (`PrimitiveComponent.SetMaterial` (`self.SpaceMesh`) 0 (`self.Material`)))

(fn `UserConstructionScript`)